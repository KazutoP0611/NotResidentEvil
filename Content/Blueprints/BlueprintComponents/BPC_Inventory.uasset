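; Inventory component that holds the player's items in a fixed-size slot array sized from NRE_PlayerController, with expandable slots.
; AddItem fills partial stacks, then empty slots, recursing on overflow and reporting any remainder, while each change refreshes its grid widget slot.
; UseItem calls an existing or spawned item actor and removes one on success; DropItem spawns a physics pickup at a camera trace.
; It also creates and opens the examination widget.
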(event Custom|Initialize
  (bind _returnvalue (Game|GetPlayerController 0))
  (bind _asnre_player_controller (Utilities|Casting|CastToNRE_PlayerController _returnvalue))
  (Utilities|Array|Resize (Variables|Default|GetInventorySlots) (Variables|/Game/GameBP/NRE_PlayerController.NRE_PlayerController_C|GetInventorySlots _asnre_player_controller))
  (Variables|Default|SetInventory%20Menu%20Ref (Variables|/Game/GameBP/NRE_PlayerController.NRE_PlayerController_C|GetInventoryMenuRef _asnre_player_controller))
  (bind _asplayer_character_l1 (Utilities|Casting|CastToPlayerCharacter_L1 (Game|GetPlayerCharacter 0)))
  (Variables|Default|SetPlayerRef _asplayer_character_l1)
  (bind _returnvalue_2 (UserInterface|CreateWidget "/Game/UMG/Inventories/W_Examination.W_Examination_C" 0 0))
  (Variables|Default|SetW_ExaminationRef _returnvalue_2)
  (Variables|/Game/GameBP/NRE_PlayerController.NRE_PlayerController_C|SetW_ExaminationWidget _asnre_player_controller (Variables|Default|GetW_ExaminationRef))
  (bind _outactors (Actor|GetAllActorsOfClass "/Game/Blueprints/Actors/Inventory/BP_Examination.BP_Examination_C"))
  (Variables|Default|SetBP_ExaminationRef (Utilities|Array|Get(acopy) _outactors))
  (Variables|/Game/UMG/Inventories/W_Examination.W_Examination_C|SetBPC_InventoryRef (Variables|Default|GetW_ExaminationRef) self))

(event Custom|UpdateExaminationWidget
  (params (Index :type Integer))
  (bind _inventory_menu_ref (Variables|Default|GetInventory%20Menu%20Ref))
  (Default|UpdateWidget (Variables|Default|GetW_ExaminationRef) Index)
  (Widget|SetVisibility _inventory_menu_ref "Collapsed")
  (Utilities|IsValid (Variables|/Game/UMG/Inventories/W_InventoryMenu.W_InventoryMenu_C|GetW_InventoryDropDown _inventory_menu_ref)
    (:Is%20Valid
      (Default|CloseDropDownMenu _inventory_menu_ref))
    (:Is%20Not%20Valid
      _))
  (UserInterface|Viewport|AddtoViewport (Variables|Default|GetW_ExaminationRef) 2)
  (Variables|/Game/GameBP/NRE_PlayerController.NRE_PlayerController_C|SetIsInventoryOpen (.AsNRE%20Player%20Controller (Utilities|Casting|CastToNRE_PlayerController (Game|GetPlayerController 0))) false))

(event EventBeginPlay
  (CallFunction|Initialize))

(event EventTick
  (params (DeltaSeconds :type Float%20%28single-precision%29)))

(fn AddItem
  (params (Item :type BP%20Inventory%20Item%20Master%20Class%20Reference) (Amount :type Integer))
  (bind (_success _index) (CallFunction|CheckforEmptySlot))
  (bind (_success_2 _index_2) (CallFunction|CheckforEmptySlot))
  (LocalVariables|SetLocalItem Item)
  (LocalVariables|SetLocalAmount Amount)
  (LocalVariables|SetLocalMaxStackAmount (.MaxStackAmount (Utilities|Struct|BreakS_ItemData (.ItemData (Utilities|GetClassDefaults (LocalVariables|GetLocalItem))))))
  (if (> (.MaxStackAmount (Utilities|Struct|BreakS_ItemData (.ItemData (Utilities|GetClassDefaults (LocalVariables|GetLocalItem))))) 1)
    (bind (_success_3 _index_3) (CallFunction|CheckforAvailableSlot (LocalVariables|GetLocalItem)))
    (if _success_3
      (LocalVariables|SetLocalIndex _index_3)
      (if (> (+ (.Amount (CallFunction|GetItemDataatIndex (LocalVariables|GetLocalIndex))) (LocalVariables|GetLocalAmount)) (LocalVariables|GetLocalMaxStackAmount))
        (LocalVariables|SetLocalAmount (- (+ (.Amount (CallFunction|GetItemDataatIndex (LocalVariables|GetLocalIndex))) (LocalVariables|GetLocalAmount)) (LocalVariables|GetLocalMaxStackAmount)))
        (Utilities|Array|SetArrayElem (Variables|Default|GetInventorySlots) (LocalVariables|GetLocalIndex) (Utilities|Struct|MakeS_InventoryItem (LocalVariables|GetLocalItem) (LocalVariables|GetLocalMaxStackAmount)))
        (CallFunction|UpdateInventorySlot (LocalVariables|GetLocalIndex))
        (bind _remainder (CallFunction|AddItem (LocalVariables|GetLocalItem) (LocalVariables|GetLocalAmount)))
        (return true _remainder)
        (else
          (Utilities|Array|SetArrayElem (Variables|Default|GetInventorySlots) (LocalVariables|GetLocalIndex) (Utilities|Struct|MakeS_InventoryItem (LocalVariables|GetLocalItem) (+ (.Amount (CallFunction|GetItemDataatIndex (LocalVariables|GetLocalIndex))) (LocalVariables|GetLocalAmount))))
          (CallFunction|UpdateInventorySlot (LocalVariables|GetLocalIndex))
          (return true 0)))
      (elif _success
        (LocalVariables|SetLocalIndex _index)
        (if (> (LocalVariables|GetLocalAmount) (LocalVariables|GetLocalMaxStackAmount))
          (Utilities|Array|SetArrayElem (Variables|Default|GetInventorySlots) (LocalVariables|GetLocalIndex) (Utilities|Struct|MakeS_InventoryItem (LocalVariables|GetLocalItem) (LocalVariables|GetLocalMaxStackAmount)))
          (CallFunction|UpdateInventorySlot (LocalVariables|GetLocalIndex))
          (bind _remainder_2 (CallFunction|AddItem (LocalVariables|GetLocalItem) (- (LocalVariables|GetLocalAmount) (LocalVariables|GetLocalMaxStackAmount))))
          (return true _remainder_2)
          (else
            (Utilities|Array|SetArrayElem (Variables|Default|GetInventorySlots) (LocalVariables|GetLocalIndex) (Utilities|Struct|MakeS_InventoryItem (LocalVariables|GetLocalItem) (LocalVariables|GetLocalAmount)))
            (CallFunction|UpdateInventorySlot (LocalVariables|GetLocalIndex))
            (return true 0)))
        (else
          (return false (LocalVariables|GetLocalAmount)))))
    (elif _success_2
      (bind _output_get (LocalVariables|SetLocalIndex _index_2))
      (Utilities|Array|SetArrayElem (Variables|Default|GetInventorySlots) _output_get (Utilities|Struct|MakeS_InventoryItem (LocalVariables|GetLocalItem) 1))
      (CallFunction|UpdateInventorySlot (LocalVariables|GetLocalIndex))
      (if (> (- (LocalVariables|GetLocalAmount) 1) 0)
        (bind _remainder_3 (CallFunction|AddItem (LocalVariables|GetLocalItem) (- (LocalVariables|GetLocalAmount) 1)))
        (return true _remainder_3)
        (else
          (return true 0)))
      (else
        (Development|PrintString "Do not have empty slot")
        (return false (LocalVariables|GetLocalAmount))))))

(fn CheckforEmptySlot
  (bind (_array_element _array_index) (Utilities|Array|ForEachLoopwithBreak (Variables|Default|GetInventorySlots) :!label _label)
    (:LoopBody
      (if (Utilities|IsValidClass (.Item (Utilities|Struct|BreakS_InventoryItem _array_element)))
        (LocalVariables|SetLocalSuccess false)
        (else
          (LocalVariables|SetLocalSuccess true)
          (LocalVariables|SetLocalIndex _array_index)
          (goto _label Break))))
    (:Completed
      (return (LocalVariables|GetLocalSuccess) (LocalVariables|GetLocalIndex)))))

(fn GetItemDataatIndex
  (params (Index :type Integer))
  (bind _inventoryslots (Variables|Default|GetInventorySlots))
  (bind _output (Utilities|Array|Get(acopy) _inventoryslots Index))
  (bind (_item _amount) (Utilities|Struct|BreakS_InventoryItem _output))
  (return _item _amount))

(fn UpdateInventorySlot
  (params (Index :type Integer))
  (Default|UpdateSlot (Utilities|Array|Get(acopy) (Variables|/Game/UMG/Inventories/W_InventoryGrid.W_InventoryGrid_C|GetSlotArray (Variables|/Game/UMG/Inventories/W_InventoryMenu.W_InventoryMenu_C|GetW_InventoryGrid (Variables|/Game/GameBP/NRE_PlayerController.NRE_PlayerController_C|GetInventoryMenuRef (.AsNRE%20Player%20Controller (Utilities|Casting|CastToNRE_PlayerController (Game|GetPlayerController 0)))))) Index)))

(fn CheckforAvailableSlot
  (params (Item :type BP%20Inventory%20Item%20Master%20Class%20Reference))
  (bind (_array_element _array_index) (Utilities|Array|ForEachLoopwithBreak (Variables|Default|GetInventorySlots) :!label _label)
    (:LoopBody
      (if (and (== (.Item (Utilities|Struct|BreakS_InventoryItem _array_element)) Item) (< (.Amount (Utilities|Struct|BreakS_InventoryItem _array_element)) (.maxstackamount (.ItemData (Utilities|GetClassDefaults Item)))))
        (LocalVariables|SetLocalSuccess true)
        (LocalVariables|SetLocalIndex _array_index)
        (goto _label Break)
        (else
          (LocalVariables|SetLocalSuccess false)
          (LocalVariables|SetLocalIndex -1))))
    (:Completed
      (return (LocalVariables|GetLocalSuccess) (LocalVariables|GetLocalIndex)))))

(fn UseItem
  (params (Index :type Integer))
  (bind _output_get (LocalVariables|SetLocalIndex Index))
  (if (> (.Amount (CallFunction|GetItemDataatIndex _output_get)) 0)
    (bind _returnvalue (Actor|GetActorOfClass (.Item (CallFunction|GetItemDataatIndex _output_get))))
    (Utilities|IsValid _returnvalue
      (:Is%20Valid
        (Default|UseItem _returnvalue)
        (if (Variables|/Game/Blueprints/Actors/Inventory/BP_InventoryItem_Master.BP_InventoryItem_Master_C|GetUseItemSuccess _returnvalue)
          (CallFunction|RemoveItem (LocalVariables|GetLocalIndex) :!label _label)
          (Default|CloseDropDownMenu (Variables|Default|GetInventory%20Menu%20Ref))))
      (:Is%20Not%20Valid
        (bind _returnvalue_2 (Game|SpawnActorfromClass (.Item (CallFunction|GetItemDataatIndex _output_get)) (Math|Transform|MakeTransform "0, 0, 0" "0, 0, 0" "1.000000,1.000000,1.000000") "Undefined" "MultiplyWithRoot" 0 0))
        (Default|UseItem _returnvalue_2)
        (if (Variables|/Game/Blueprints/Actors/Inventory/BP_InventoryItem_Master.BP_InventoryItem_Master_C|GetUseItemSuccess _returnvalue_2)
          (goto _label))))))

(fn RemoveItem
  (params (Index :type Integer))
  (bind (_item _amount) (CallFunction|GetItemDataatIndex Index))
  (if (> _amount 1)
    (Utilities|Array|SetArrayElem (Variables|Default|GetInventorySlots) Index (Utilities|Struct|MakeS_InventoryItem _item (- _amount 1)))
    (else
      (Utilities|Array|SetArrayElem (Variables|Default|GetInventorySlots) Index (Utilities|Struct|MakeS_InventoryItem 0 0))))
  (CallFunction|UpdateInventorySlot Index))

(fn DropItem
  (params (Index :type Integer))
  (bind _playerref (Variables|Default|GetPlayerRef))
  (bind _camera (Variables|/Game/GameBP/Level1/PlayerCharacter_L1.PlayerCharacter_L1_C|GetCamera _playerref))
  (bind _returnvalue (Transformation|GetWorldLocation _camera))
  (bind _output_get (LocalVariables|SetLocalIndex Index))
  (LocalVariables|SetLocalAmount (.Amount (CallFunction|GetItemDataatIndex _output_get)))
  (LocalVariables|SetLocalItemClass (.Item (CallFunction|GetItemDataatIndex _output_get)))
  (if (> (LocalVariables|GetLocalAmount) 0)
    (for _index (range 0 (- (LocalVariables|GetLocalAmount) 1))
      (CallFunction|RemoveItem (LocalVariables|GetLocalIndex)))
    (Default|CloseDropDownMenu (Variables|Default|GetInventory%20Menu%20Ref))
    (bind _outhit (Collision|LineTraceByChannel _returnvalue (+ _returnvalue (* (Math|Vector|GetForwardVector _camera) (Math|Conversions|ToVector(Float) 2e+02))) "TraceTypeQuery1" false 0 "None"))
    (bind _returnvalue_2 (Game|SpawnActorfromClass (.PickUpActor (Utilities|Struct|BreakS_ItemData (.ItemData (Utilities|GetClassDefaults (LocalVariables|GetLocalItemClass))))) (Math|Transform|MakeTransform (select (.bBlockingHit (Collision|BreakHitResult _outhit)) (.Location (Collision|BreakHitResult _outhit)) (.TraceEnd (Collision|BreakHitResult _outhit))) "0, 0, 0" "1.000000,1.000000,1.000000") "Undefined" "MultiplyWithRoot" 0 0))
    (Variables|/Game/Blueprints/Actors/Inventory/PickupActors/BP_PIckupActor_Master.BP_PIckupActor_Master_C|SetAmount _returnvalue_2 (LocalVariables|GetLocalAmount))
    (Physics|SetSimulatePhysics (Variables|/Game/Blueprints/Actors/Inventory/PickupActors/BP_PIckupActor_Master.BP_PIckupActor_Master_C|GetStaticMesh _returnvalue_2) true)))

(fn AddMoreSlots
  (params (Amount :type Integer))
  (bind _returnvalue (Game|GetPlayerController 0))
  (bind _inventory_menu_ref (Variables|Default|GetInventory%20Menu%20Ref))
  (bind _asnre_player_controller (Utilities|Casting|CastToNRE_PlayerController _returnvalue))
  (bind _w_inventorygrid (Variables|/Game/UMG/Inventories/W_InventoryMenu.W_InventoryMenu_C|GetW_InventoryGrid _inventory_menu_ref))
  (bind _output_get (Variables|/Game/GameBP/NRE_PlayerController.NRE_PlayerController_C|SetInventorySlots _asnre_player_controller (+ Amount (Variables|/Game/GameBP/NRE_PlayerController.NRE_PlayerController_C|GetInventorySlots _asnre_player_controller))))
  (Utilities|Array|Resize (Variables|Default|GetInventorySlots) _output_get)
  (Default|AddMoreSlots _w_inventorygrid Amount)
  (for _array_element (Variables|/Game/UMG/Inventories/W_InventoryGrid.W_InventoryGrid_C|GetSlotArray _w_inventorygrid)
    (Default|Initialize _array_element _inventory_menu_ref)))