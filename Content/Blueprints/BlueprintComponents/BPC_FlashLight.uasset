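; Flashlight component that manages a battery-powered light, which it takes from the player on Initialize and starts switched off.
; Toggling on requires charge and starts a looping timer that drains the battery, switching the light off at the minimum level.
; Battery changes update the light's IES brightness scale through a clamped mapping, so it dims below a set charge threshold.
; AddBatteryLife recharges within limits, while battery status is printed as on-screen strings.
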(event EventBeginPlay)

(event EventTick
  (params (DeltaSeconds :type Float%20%28single-precision%29)))

(fn ToggleFlashLight
  (if (Variables|/Script/Engine.SceneComponent|GetbVisible (Variables|Default|GetFlashLight))
    (CallFunction|SetActiveFlashLight false)
    (elif (> (Variables|Default|GetCurrentBatteryLevel) (Variables|Default|GetMinBatteryLevel))
      (CallFunction|SetActiveFlashLight true)
      (else
        (Development|PrintString "Battery is dead")))))

(fn Initialize
  (params (Player :type Player%20Character%20L1%20Object%20Reference))
  (bind _output_get (Variables|Default|SetPlayer Player))
  (Variables|Default|SetFlashLight (Variables|/Game/GameBP/Level1/PlayerCharacter_L1.PlayerCharacter_L1_C|GetFlashLight _output_get))
  (CallFunction|SetActiveFlashLight false))

(fn DepleteBatteryLife
  (bind _output_get (Variables|Default|SetCurrentBatteryLevel (Math|Float|Clamp(Float) (- (Variables|Default|GetCurrentBatteryLevel) (Variables|Default|GetDepletionAmount)) (Variables|Default|GetMinBatteryLevel) (Variables|Default|GetMaxBatteryLevel))))
  (CallFunction|SetIntensity)
  (if (and (<= _output_get (Variables|Default|GetMinBatteryLevel)) (Variables|/Script/Engine.SceneComponent|GetbVisible (Variables|Default|GetFlashLight)))
    (CallFunction|ToggleFlashLight)
    (else
      (Development|PrintString (Utilities|String|ToString(Float) _output_get)))))

(fn AddBatteryLife
  (params (Amount :type Float%20%28double-precision%29))
  (Variables|Default|SetCurrentBatteryLevel (Math|Float|Clamp(Float) (+ Amount (Variables|Default|GetCurrentBatteryLevel)) (Variables|Default|GetMinBatteryLevel) (Variables|Default|GetMaxBatteryLevel)))
  (CallFunction|SetIntensity))

(fn SetActiveFlashLight
  (params (Active :type Boolean))
  (Rendering|SetVisibility (Variables|Default|GetFlashLight) Active false)
  (if Active
    (CallFunction|SetIntensity)
    (Utilities|Time|SetTimerbyFunctionName 0 "DepleteBatteryLife" (Variables|Default|GetDepletionSpeed) true)
    (else
      (Utilities|Time|ClearTimerbyFunctionName 0 "DepleteBatteryLife"))))

(fn SetIntensity
  (Class|LightComponent|SetIESBrightnessScale (Variables|Default|GetFlashLight) (Math|Float|MapRangeClamped (Variables|Default|GetCurrentBatteryLevel) (Variables|Default|GetMinBatteryLevel) (Variables|Default|GetLostLightIntensityAtBatteryLevel) 0.0 1.0)))