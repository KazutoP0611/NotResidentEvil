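; Interactable combination lock actor that opens and destroys itself once its four dials match LockCombination.
; BeginPlay spawns BP_LockDial actors on skeletal mesh sockets, passing each its index and a lock reference.
; Interact blends to the lock camera, disables movement and enables cursor, dial arrows and widget-interaction clicks until exit restores player control.
; CheckEveryTurn tests the code, then plays the open animation, exits the view and removes lock and dials.
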(event Custom|Exit%20Lock%20View
  (bind _playercontrollerref (Variables|Default|GetPlayerControllerRef))
  (for _array_element (Variables|Default|GetDial)
    (Default|ToggleArrows _array_element false)
    (Input|DisableInput _playercontrollerref)
    (Variables|/Script/Engine.PlayerController|SetbShowMouseCursor _playercontrollerref false)
    (Game|Player|SetViewTargetwithBlend (Variables|Default|GetPlayerControllerRef) (Game|GetPlayerCharacter 0) (Variables|Default|GetCameraBlendTime) "VTBlend_Linear" 0.0 false)
    (Variables|/Game/GameBP/NRE_PlayerController.NRE_PlayerController_C|SetCanOpenInventory (Variables|Default|GetPlayerControllerRef) true)
    (Input|ResetIgnoreLookInput (Variables|Default|GetPlayerControllerRef))
    (Utilities|FlowControl|Delay (Variables|Default|GetCameraBlendTime))
    (Pawn|Components|CharacterMovement|SetMovementMode (Variables|/Script/Engine.Character|GetCharacterMovement (Game|GetPlayerCharacter 0)) "MOVE_Walking" 0)))

(event Custom|Check%20Every%20Turn
  (bind _success (CallFunction|CheckCode))
  (if _success
    (Components|Animation|PlayAnimation (Variables|Default|GetLockSkeletonMesh) "/Game/Props/Animations/LockOpen.LockOpen" false)
    (Utilities|FlowControl|Delay 1.5)
    (CallFunction|ExitLockView)
    (Utilities|FlowControl|Delay 1.0)
    (for _array_element (Variables|Default|GetDial)
      (Actor|DestroyActor _array_element))
    (Actor|DestroyActor)))

(event EventBeginPlay
  (Variables|Default|SetPlayerControllerRef (.AsNRE%20Player%20Controller (Utilities|Casting|CastToNRE_PlayerController (Game|GetPlayerController 0))))
  (for _index (range 0 3)
    (bind _returnvalue (Game|SpawnActorfromClass "/Game/Blueprints/Actors/BP_LockDial.BP_LockDial_C" (Math|Transform|MakeTransform "0, 0, 0" "0, 0, 0" "1.000000,1.000000,1.000000") "AlwaysSpawn" "MultiplyWithRoot" 0 _index self 0))
    (Utilities|Array|Add (Variables|Default|GetDial) _returnvalue)
    (Transformation|AttachComponentToComponent _returnvalue (Variables|Default|GetLockSkeletonMesh) (Utilities|String|StringToName (Utilities|String|BuildString(Name) "DialBone" (Utilities|String|ToString(Integer) (+ _index 1)) "Socket" "")) "SnapToTarget" "KeepWorld" "KeepWorld" true)))

(event EventInteract
  (bind _playercontrollerref (Variables|Default|GetPlayerControllerRef))
  (Variables|/Game/GameBP/NRE_PlayerController.NRE_PlayerController_C|SetCanOpenInventory (Variables|Default|GetPlayerControllerRef) false)
  (Game|Player|SetViewTargetwithBlend (Variables|Default|GetPlayerControllerRef) (Components|GetOwner (Variables|Default|GetCamera)) (Variables|Default|GetCameraBlendTime) "VTBlend_Linear" 0.0 false)
  (Pawn|Components|CharacterMovement|DisableMovement (Variables|/Script/Engine.Character|GetCharacterMovement (Game|GetPlayerCharacter 0)))
  (Input|SetIgnoreLookInput (Variables|Default|GetPlayerControllerRef) false)
  (Utilities|FlowControl|Delay (Variables|Default|GetCameraBlendTime))
  (Input|EnableInput _playercontrollerref)
  (Variables|/Script/Engine.PlayerController|SetbShowMouseCursor _playercontrollerref true)
  (for _array_element (Variables|Default|GetDial)
    (Default|ToggleArrows _array_element true)))

(event Input|ActionEvents|InputActionInteraction
  (params (Key :type Key%20Structure :default "None"))
  (:Pressed
    (CallFunction|ExitLockView)))

(event Input|ActionEvents|InputActionLeftMouseButton
  (params (Key :type Key%20Structure :default "None"))
  (bind _widgetinteraction (Variables|Default|GetWidgetInteraction))
  (:Pressed
    (Class|WidgetInteractionComponent|PressPointerKey _widgetinteraction "LeftMouseButton"))
  (:Released
    (Class|WidgetInteractionComponent|ReleasePointerKey _widgetinteraction "LeftMouseButton")))

(event Input|KeyboardEvents|Escape
  (params (Key :type Key%20Structure :default "None"))
  (:Pressed
    (CallFunction|ExitLockView)))

(event Input|KeyboardEvents|Backspace
  (params (Key :type Key%20Structure :default "None"))
  (:Pressed
    (CallFunction|ExitLockView)))

(fn ConstructionScript
  (Components|Box|SetBoxExtent (Variables|Default|GetBox) (Variables|Default|GetBoxExtent) true)
  (Transformation|SetRelativeLocation (Variables|Default|GetBox) (Variables|Default|GetBoxPosition) false false))

(fn CheckCode
  (bind (_array_element _array_index) (Utilities|Array|ForEachLoopwithBreak (Variables|Default|GetDial) :!label _label)
    (:LoopBody
      (if (== (Variables|/Game/Blueprints/Actors/BP_LockDial.BP_LockDial_C|GetNumber _array_element) (Utilities|Array|Get(acopy) (Variables|Default|GetLockCombination) _array_index))
        (LocalVariables|SetLocalSuccess true)
        (else
          (LocalVariables|SetLocalSuccess false)
          (goto _label Break))))
    (:Completed
      (return (LocalVariables|GetLocalSuccess)))))