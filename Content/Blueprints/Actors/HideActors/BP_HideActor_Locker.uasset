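; BP_HideActor_Locker is a hiding-spot locker whose door swings open and shut around the player's hide sequence.
; Interact blocks reuse, rotates the door open on a timeline, then calls the parent interaction after a short delay.
; When the parent's finished-moving dispatcher fires, the door closes and interaction re-enables.
; EnemyFound disables interaction and door collision and swings the door open through a separate timeline.
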(event Custom|Close%20Door
  (bind _alpha (Timeline|Timeline PlayFromStart)
    (:Update
      (Transformation|SetRelativeRotation (Variables|Default|GetLockerDoor) (Math|Rotator|MakeRotator 0.0 0.0 (Math|Float|Lerp 9e+01 0.0 _alpha)) false false))
    (:Finished
      (Variables|Default|SetCanInteract true))))

(event Custom|FinishededMovingED_Event
  (Utilities|FlowControl|Delay 0.15)
  (CallFunction|CloseDoor))

(event EventEnemyFound
  (Variables|Default|SetCanInteract false)
  (Collision|SetCollisionEnabled (Variables|Default|GetLockerDoor) "NoCollision")
  (bind _alpha (Timeline|AIOpenDoor PlayFromStart)
    (:Update
      (Transformation|SetRelativeRotation (Variables|Default|GetLockerDoor) (Math|Rotator|MakeRotator 0.0 0.0 (Math|Float|Lerp 0.0 9e+01 _alpha)) false false))
    (:Finished
      (Utilities|FlowControl|Delay 0.12))))

(event EventInteract
  (if (Variables|Default|GetCanInteract)
    (Variables|Default|SetCanInteract false)
    (bind _alpha (Timeline|OpenLockerDoor PlayFromStart)
      (:Update
        (Transformation|SetRelativeRotation (Variables|Default|GetLockerDoor) (Math|Rotator|MakeRotator 0.0 0.0 (Math|Float|Lerp 0.0 9e+01 _alpha)) false false))
      (:Finished
        (Utilities|FlowControl|Delay 0.12)
        (|CallParentFunction)))))

(event EventBeginPlay
  (|CallParentFunction)
  (EventDispatchers|AssignFinishededMovingED (delegate Custom|FinishededMovingED_Event)))

(fn ConstructionScript
  (|CallParentFunction))