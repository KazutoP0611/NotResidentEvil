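; Hiding spot actor that Interact uses to move the player into or out of hiding.
; A looping timer, set at the current frame delta, interpolates the player at constant speed to the hiding or exit position.
; Entering alerts the AIC_Classic enemy AI and disables collision and movement.
; Arrival fires a finished dispatcher and toggles IsHiding; exiting then notifies the AI and restores both. EnemyFound is empty.
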(event Custom|Move%20Character
  (bind _playerref (Variables|Default|GetPlayerRef))
  (Transformation|SetActorTransform _playerref (Math|Transform|MakeTransform (Math|Interpolation|VInterptoConstant (Transformation|GetActorLocation _playerref) (Transformation|GetWorldLocation (select (Variables|/Game/GameBP/Level1/PlayerCharacter_L1.PlayerCharacter_L1_C|GetIsHiding (Variables|Default|GetPlayerRef)) (Variables|Default|GetExitPosition) (Variables|Default|GetHidingPosition))) (Utilities|Time|GetWorldDeltaSeconds) 1e+03) "0, 0, 0" "1.000000,1.000000,1.000000"))
  (if (Utilities|Operators|EqualEqual (Transformation|GetActorLocation (Variables|Default|GetPlayerRef)) (Transformation|GetWorldLocation (select (Variables|/Game/GameBP/Level1/PlayerCharacter_L1.PlayerCharacter_L1_C|GetIsHiding (Variables|Default|GetPlayerRef)) (Variables|Default|GetExitPosition) (Variables|Default|GetHidingPosition))) 0.01)
    (Utilities|Time|ClearandInvalidateTimerbyHandle (stale EventInteract _returnvalue_3))
    (Utilities|Time|ClearandInvalidateTimerbyHandle (stale EventInteract _returnvalue))
    (CallFunction|FinishMoving)))

(event Custom|Finish%20Moving
  (bind _playerref (Variables|Default|GetPlayerRef))
  (bind _playerref_2 (Variables|Default|GetPlayerRef))
  (Default|CallFinishededMovingED)
  (bind _output_get (Variables|/Game/GameBP/Level1/PlayerCharacter_L1.PlayerCharacter_L1_C|SetIsHiding _playerref (not (Variables|/Game/GameBP/Level1/PlayerCharacter_L1.PlayerCharacter_L1_C|GetIsHiding _playerref))))
  (if (not _output_get)
    (bind _asaic_classic (Utilities|Casting|CastToAIC_ClassicClass "/Game/AI/ClassicHorrorAI/AIC_Classic.AIC_Classic_C"))
    (bind _returnvalue (Actor|GetActorOfClass _asaic_classic))
    (Class|BPIPlayerHiding|LeftHidingSpot(Message) _returnvalue)
    (Collision|SetActorEnableCollision _playerref_2 true)
    (Pawn|Components|CharacterMovement|SetMovementMode (Variables|/Script/Engine.Character|GetCharacterMovement _playerref_2) "MOVE_Walking" 0)))

(event Custom|EnemyFound)

(event EventBeginPlay
  (bind _asplayer_character_l1 (Utilities|Casting|CastToPlayerCharacter_L1 (Game|GetPlayerCharacter 0)))
  (Variables|Default|SetPlayerRef _asplayer_character_l1))

(event EventInteract
  (bind _playerref (Variables|Default|GetPlayerRef))
  (if (Variables|/Game/GameBP/Level1/PlayerCharacter_L1.PlayerCharacter_L1_C|GetIsHiding (Variables|Default|GetPlayerRef))
    (bind _returnvalue (Utilities|Time|SetTimerbyEvent (delegate Custom|Move%20Character) (Utilities|Time|GetWorldDeltaSeconds) true))
    (else
      (bind _asaic_classic (Utilities|Casting|CastToAIC_ClassicClass "/Game/AI/ClassicHorrorAI/AIC_Classic.AIC_Classic_C"))
      (bind _returnvalue_2 (Actor|GetActorOfClass _asaic_classic))
      (Class|BPIPlayerHiding|EnemySaw(Message) _returnvalue_2 self)
      (Collision|SetActorEnableCollision _playerref false)
      (Pawn|Components|CharacterMovement|DisableMovement (Variables|/Script/Engine.Character|GetCharacterMovement _playerref))
      (bind _returnvalue_3 (Utilities|Time|SetTimerbyEvent (delegate Custom|Move%20Character) (Utilities|Time|GetWorldDeltaSeconds) true)))))

(fn ConstructionScript)