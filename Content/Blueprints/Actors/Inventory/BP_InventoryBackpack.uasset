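; BP_InventoryBackpack is a world pickup that adds slots to the player's inventory component, then destroys itself.
; A sphere overlap with PlayerCharacter_L1 starts per-tick updates, with a visibility trace from the mesh to the player camera.
; With a clear line of sight, the prompt widget shows and turns toward the camera.
; Within pickup distance, the prompt toggles and input is enabled for the Interaction action.
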(event OnComponentBeginOverlap(Sphere)
  (params (OverlappedComponent :type Primitive%20Component%20Object%20Reference) (OtherActor :type Actor%20Object%20Reference) (OtherComp :type Primitive%20Component%20Object%20Reference) (OtherBodyIndex :type Integer) (bFromSweep :type Boolean) (SweepResult :type Hit%20Result%20Structure%20%28by%20ref%29))
  (bind _asplayer_character_l1 (Utilities|Casting|CastToPlayerCharacter_L1 OtherActor))
  (Variables|Default|SetPlayerRef _asplayer_character_l1)
  (Rendering|SetVisibility (Variables|Default|GetPickupWidget) true false)
  (Variables|Default|SetUpdateActor true))

(event OnComponentEndOverlap(Sphere)
  (params (OverlappedComponent :type Primitive%20Component%20Object%20Reference) (OtherActor :type Actor%20Object%20Reference) (OtherComp :type Primitive%20Component%20Object%20Reference) (OtherBodyIndex :type Integer))
  (Utilities|Casting|CastToPlayerCharacter_L1 OtherActor)
  (Rendering|SetVisibility (Variables|Default|GetPickupWidget) false false)
  (Variables|Default|SetUpdateActor false)
  (Input|DisableInput (Game|GetPlayerController 0)))

(event EventBeginPlay)

(event Collision|EventActorBeginOverlap
  (params (OtherActor :type Actor%20Object%20Reference)))

(event EventTick
  (params (DeltaSeconds :type Float%20%28single-precision%29))
  (bind _returnvalue (Game|GetPlayerController 0))
  (bind _pickupwidget (Variables|Default|GetPickupWidget))
  (Transformation|SetWorldLocation (Variables|Default|GetPickupWidget) (+ (Transformation|GetWorldLocation (Variables|Default|GetStaticMesh)) (Math|Vector|MakeVector 0.0 0.0 (Variables|Default|GetPromptWidgetDistance))) false false)
  (if (Variables|Default|GetUpdateActor)
    (bind (_outhit _returnvalue_2) (Collision|LineTraceByChannel (Transformation|GetWorldLocation (Variables|Default|GetStaticMesh)) (Transformation|GetWorldLocation (Variables|/Game/GameBP/Level1/PlayerCharacter_L1.PlayerCharacter_L1_C|GetCamera (Variables|Default|GetPlayerRef))) "TraceTypeQuery1" false 0 "None"))
    (if (not _returnvalue_2)
      (Rendering|SetVisibility _pickupwidget true false)
      (Transformation|SetWorldRotation (Variables|Default|GetPickupWidget) (Math|Rotator|FindLookatRotation (Transformation|GetWorldLocation (Variables|Default|GetPickupWidget)) (Transformation|GetWorldLocation (Variables|/Game/GameBP/Level1/PlayerCharacter_L1.PlayerCharacter_L1_C|GetCamera (Variables|Default|GetPlayerRef)))) false false)
      (Default|TogglePrompt (.AsW%20PIck%20Up%20Prompt (Utilities|Casting|CastToW_PIckUpPrompt (UserInterface|GetUserWidgetObject (Variables|Default|GetPickupWidget)))) (<= (Math|Vector|VectorLength (- (.TraceStart (Collision|BreakHitResult _outhit)) (.TraceEnd (Collision|BreakHitResult _outhit)))) (Variables|Default|GetPickUpDistance)))
      (if (<= (Math|Vector|VectorLength (- (.TraceStart (Collision|BreakHitResult _outhit)) (.TraceEnd (Collision|BreakHitResult _outhit)))) (Variables|Default|GetPickUpDistance))
        (Input|EnableInput _returnvalue)
        (else
          (Input|DisableInput _returnvalue)))
      (else
        (Rendering|SetVisibility _pickupwidget false false)
        (Input|DisableInput (Game|GetPlayerController 0))))))

(event Input|ActionEvents|InputActionInteraction
  (params (Key :type Key%20Structure :default "None"))
  (:Pressed
    (Default|AddMoreSlots (Variables|/Game/GameBP/Level1/PlayerCharacter_L1.PlayerCharacter_L1_C|GetBPC_Inventory (Variables|Default|GetPlayerRef)) (Variables|Default|GetAmountOfSlots))
    (Actor|DestroyActor)))

(fn ConstructionScript)