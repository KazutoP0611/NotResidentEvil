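; BP_CameraController is an interactable station that lets the player view the level's security cameras.
; On BeginPlay it gathers every BP_SecurityCamera, then Interact takes input from the player character, hides the main HUD and blends the view to the current camera.
; Space bar cycles through the cameras with wraparound.
; Return, Interaction or a repeat Interact restores the player's input, HUD and view.
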(event Custom|LeaveCameraController
  (bind _returnvalue (Game|GetPlayerController 0))
  (Variables|Default|SetIsViewing false)
  (Input|DisableInput _returnvalue)
  (Input|ResetIgnoreLookInput _returnvalue)
  (Widget|SetVisibility (Variables|/Game/GameBP/Level1/PlayerCharacter_L1.PlayerCharacter_L1_C|GetMainHUDRef (.AsPlayer%20Character%20L1 (Utilities|Casting|CastToPlayerCharacter_L1 (Game|GetPlayerCharacter 0)))) "SelfHitTestInvisible")
  (Input|EnableInput (Game|GetPlayerCharacter 0) (Game|GetPlayerController 0))
  (Game|Player|SetViewTargetwithBlend (Game|GetPlayerController 0) (Game|GetPlayerCharacter 0) 0.0 "VTBlend_Linear" 0.0 false))

(event EventInteract
  (bind _returnvalue (Game|GetPlayerController 0))
  (if (Variables|Default|GetIsViewing)
    (CallFunction|LeaveCameraController)
    (else
      (Variables|Default|SetIsViewing true)
      (Input|DisableInput (Game|GetPlayerCharacter 0) _returnvalue)
      (Input|SetIgnoreLookInput _returnvalue true)
      (Widget|SetVisibility (Variables|/Game/GameBP/Level1/PlayerCharacter_L1.PlayerCharacter_L1_C|GetMainHUDRef (.AsPlayer%20Character%20L1 (Utilities|Casting|CastToPlayerCharacter_L1 (Game|GetPlayerCharacter 0)))) "Hidden")
      (Input|EnableInput (Game|GetPlayerController 0))
      (CallFunction|ViewThroughCameras))))

(event EventBeginPlay
  (bind _outactors (Actor|GetAllActorsOfClass "/Game/Blueprints/Actors/SecurityCamera/BP_SecurityCamera.BP_SecurityCamera_C"))
  (Variables|Default|SetSecurityCameras _outactors))

(event Input|ActionEvents|InputActionReturn
  (params (Key :type Key%20Structure :default "None"))
  (:Pressed
    (CallFunction|LeaveCameraController)))

(event Input|ActionEvents|InputActionInteraction
  (params (Key :type Key%20Structure :default "None"))
  (:Pressed
    (CallFunction|LeaveCameraController)))

(event Input|KeyboardEvents|SpaceBar
  (params (Key :type Key%20Structure :default "None"))
  (:Pressed
    (Variables|Default|SetCurrentCameraIndex (select (> (+ (Variables|Default|GetCurrentCameraIndex) 1) (- (Utilities|Array|Length (Variables|Default|GetSecurityCameras)) 1)) 0 (+ (Variables|Default|GetCurrentCameraIndex) 1)))
    (CallFunction|ViewThroughCameras)))

(fn ConstructionScript)

(fn ViewThroughCameras
  (Game|Player|SetViewTargetwithBlend (Game|GetPlayerController 0) (Utilities|Array|Get(acopy) (Variables|Default|GetSecurityCameras) (Variables|Default|GetCurrentCameraIndex)) 0.0 "VTBlend_Linear" 0.0 false)
  (return))