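; Interactable door actor that swings open or closed each time it receives an Interact event.
; An IsClosed flag toggles on each interaction and plays or reverses a single timeline.
; The timeline's alpha drives a lerp on the door mesh's relative yaw, rotating it a quarter turn between closed and open.
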(event EventBeginPlay
  (|CallParentFunction) ; This node is disabled and will not be called.\nDrag off pins to build functionality.
)

(event Collision|EventActorBeginOverlap
  (params (OtherActor :type Actor%20Object%20Reference))
  (|CallParentFunction OtherActor) ; This node is disabled and will not be called.\nDrag off pins to build functionality.
)

(event EventTick
  (params (DeltaSeconds :type Float%20%28single-precision%29))
  (|CallParentFunction DeltaSeconds) ; This node is disabled and will not be called.\nDrag off pins to build functionality.
)

(event EventInteract
  (if (Variables|Default|GetIsClosed)
    (Variables|Default|SetIsClosed false)
    (bind _alpha (Timeline|Timeline_OpenDoor Play)
      (:Update
        (Transformation|SetRelativeRotation (Variables|Default|GetStaticMesh_Door) (Math|Rotator|MakeRotator 0.0 0.0 (Math|Float|Lerp 0.0 9e+01 _alpha)) false false)))
    (else
      (Variables|Default|SetIsClosed true)
      (Timeline|Timeline_OpenDoor Reverse))))

(fn ConstructionScript
  (|CallParentFunction))