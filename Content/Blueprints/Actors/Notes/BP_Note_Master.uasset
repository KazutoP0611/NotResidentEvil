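; Readable note actor that the player can examine up close, with front and back text applied in the construction script.
; Entering its sphere starts a per-tick visibility trace to the player camera, showing a camera-facing prompt when unobstructed and enabling input within pickup distance.
; Pressing Interaction creates the examination widget, if none is valid, passing it this note and the BP_NoteExamination actor found at BeginPlay.
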(event OnComponentBeginOverlap(Sphere)
  (params (OverlappedComponent :type Primitive%20Component%20Object%20Reference) (OtherActor :type Actor%20Object%20Reference) (OtherComp :type Primitive%20Component%20Object%20Reference) (OtherBodyIndex :type Integer) (bFromSweep :type Boolean) (SweepResult :type Hit%20Result%20Structure%20%28by%20ref%29))
  (bind _asplayer_character_l1 (Utilities|Casting|CastToPlayerCharacter_L1 OtherActor))
  (Variables|Default|SetPlayerRef _asplayer_character_l1)
  (Rendering|SetVisibility (Variables|Default|GetPromptWidget) true false)
  (Variables|Default|SetUpdateActor true))

(event OnComponentEndOverlap(Sphere)
  (params (OverlappedComponent :type Primitive%20Component%20Object%20Reference) (OtherActor :type Actor%20Object%20Reference) (OtherComp :type Primitive%20Component%20Object%20Reference) (OtherBodyIndex :type Integer))
  (Utilities|Casting|CastToPlayerCharacter_L1 OtherActor)
  (Rendering|SetVisibility (Variables|Default|GetPromptWidget) false false)
  (Variables|Default|SetUpdateActor false)
  (Input|DisableInput (Game|GetPlayerController 0)))

(event EventBeginPlay
  (bind _outactors (Actor|GetAllActorsOfClass "/Game/Blueprints/Actors/Notes/BP_NoteExamination.BP_NoteExamination_C"))
  (Variables|Default|SetBP_NoteExaminationRef (Utilities|Array|Get(acopy) _outactors)))

(event Collision|EventActorBeginOverlap
  (params (OtherActor :type Actor%20Object%20Reference)))

(event EventTick
  (params (DeltaSeconds :type Float%20%28single-precision%29))
  (bind _returnvalue (Game|GetPlayerController 0))
  (bind _promptwidget (Variables|Default|GetPromptWidget))
  (Transformation|SetWorldLocation (Variables|Default|GetPromptWidget) (+ (Transformation|GetWorldLocation (Variables|Default|GetPaperMesh)) (Math|Vector|MakeVector 0.0 0.0 (Variables|Default|GetPromptWidegetDistance))) false false)
  (if (Variables|Default|GetUpdateActor)
    (bind (_outhit _returnvalue_2) (Collision|LineTraceByChannel (Transformation|GetWorldLocation (Variables|Default|GetPaperMesh)) (Transformation|GetWorldLocation (Variables|/Game/GameBP/Level1/PlayerCharacter_L1.PlayerCharacter_L1_C|GetCamera (Variables|Default|GetPlayerRef))) "TraceTypeQuery1" false 0 "None"))
    (if (not _returnvalue_2)
      (Rendering|SetVisibility _promptwidget true false)
      (Transformation|SetWorldRotation (Variables|Default|GetPromptWidget) (Math|Rotator|FindLookatRotation (Transformation|GetWorldLocation (Variables|Default|GetPromptWidget)) (Transformation|GetWorldLocation (Variables|/Game/GameBP/Level1/PlayerCharacter_L1.PlayerCharacter_L1_C|GetCamera (Variables|Default|GetPlayerRef)))) false false)
      (Default|TogglePrompt (.AsW%20PIck%20Up%20Prompt (Utilities|Casting|CastToW_PIckUpPrompt (UserInterface|GetUserWidgetObject (Variables|Default|GetPromptWidget)))) (<= (Math|Vector|VectorLength (- (.TraceStart (Collision|BreakHitResult _outhit)) (.TraceEnd (Collision|BreakHitResult _outhit)))) (Variables|Default|GetPickUpDistance)))
      (if (<= (Math|Vector|VectorLength (- (.TraceStart (Collision|BreakHitResult _outhit)) (.TraceEnd (Collision|BreakHitResult _outhit)))) (Variables|Default|GetPickUpDistance))
        (Input|EnableInput _returnvalue)
        (else
          (Input|DisableInput _returnvalue)))
      (else
        (Rendering|SetVisibility _promptwidget false false)
        (Input|DisableInput (Game|GetPlayerController 0))))))

(event Input|ActionEvents|InputActionInteraction
  (params (Key :type Key%20Structure :default "None"))
  (:Pressed
    (Utilities|IsValid (Variables|Default|GetW_ExaminationNoteRef)
      (:Is%20Not%20Valid
        (bind _returnvalue (UserInterface|CreateWidget "/Game/UMG/W_NoteExamination.W_NoteExamination_C" 0 (Variables|Default|GetBP_NoteExaminationRef)))
        (bind _output_get (Variables|Default|SetW_ExaminationNoteRef _returnvalue))
        (Default|UpdateWidget _output_get self)
        (UserInterface|Viewport|AddtoViewport _output_get 0)))))

(fn ConstructionScript
  (Rendering|Components|TextRender|SetText (Variables|Default|GetNoteText) (Variables|Default|GetNoteText%28Text%29))
  (Rendering|Components|TextRender|SetText (Variables|Default|GetBackNoteText) (Variables|Default|GetBackNoteText%28Text%29)))